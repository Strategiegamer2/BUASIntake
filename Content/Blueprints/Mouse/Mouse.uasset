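; Mouse Blueprint that lets the player left-click PushCube actors to turn on their physics.
; A click line-traces from the deprojected cursor on the Visibility channel and checks that the hit actor's class is PushCube.
; The hit cube teleports to X zero, keeping Y and Z, then simulates physics constrained to the YZ plane.
; BeginPlay also caches a PushCube reference, which the click logic does not use.
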(event EventBeginPlay
  (bind _returnvalue (Actor|GetActorOfClass "/Game/Blueprints/PushCube.PushCube_C"))
  (Variables|Default|SetPuchCubeRef _returnvalue))

(event Input|MouseEvents|LeftMouseButton
  (params (Key :type Key%20Structure :default "None"))
  (bind _returnvalue (Game|GetPlayerController 0))
  (bind (_worldlocation _worlddirection) (Game|Player|ConvertMouseLocationToWorldSpace _returnvalue))
  (:Pressed
    (bind _outhit (Collision|LineTraceByChannel _worldlocation (+ _worldlocation (* _worlddirection 1e+04)) "TraceTypeQuery1" false 0 "None"))
    (if (== (Utilities|GetClass (.hitactor _outhit)) "/Game/Blueprints/PushCube.PushCube_C")
      (Transformation|SetWorldLocation (Variables|/Script/Engine.Actor|GetRootComponent (.hitactor _outhit)) (Math|Vector|MakeVector 0.0 (.y (Transformation|GetWorldLocation (Variables|/Script/Engine.Actor|GetRootComponent (.hitactor _outhit)))) (.z (Transformation|GetWorldLocation (Variables|/Script/Engine.Actor|GetRootComponent (.hitactor _outhit))))) false true)
      (bind _aspush_cube (Utilities|Casting|CastToPushCube (.hitactor _outhit)))
      (Physics|SetSimulatePhysics (Variables|/Game/Blueprints/PushCube.PushCube_C|GetCube _aspush_cube) true)
      (Class|PrimitiveComponent|SetConstraintMode (Variables|/Game/Blueprints/PushCube.PushCube_C|GetCube _aspush_cube) "YZPlane"))))

(fn ConstructionScript)