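; Level 2 finish flag that times the run with a one-second looping timer and ends the level on overlap.
; Two trigger boxes each destroy the other, then share a one-shot sequence that freezes the character, moves the follow camera and drops the flag as it turns green.
; After a delay, Box shows the completion widget and Box1 the Tip variant, both receiving the seconds and switching to UI-only input with a visible cursor.
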(event OnComponentBeginOverlap(Box)
  (params (OverlappedComponent :type Primitive%20Component%20Object%20Reference) (OtherActor :type Actor%20Object%20Reference) (OtherComp :type Primitive%20Component%20Object%20Reference) (OtherBodyIndex :type Integer) (bFromSweep :type Boolean) (SweepResult :type Hit%20Result%20Structure%20%28by%20ref%29))
  (bind _returnvalue (Game|GetPlayerController 0))
  (bind _flag (Variables|Default|GetFlag))
  (bind _relativelocation (Variables|/Script/Engine.SceneComponent|GetRelativeLocation _flag))
  ;[0.2008 0.6135 0.1357] Here the win-screen is created, we tell it how many seconds it took to complete. Then it's added to the screen and we make sure that the player can see their mouse and restart the level
  (Components|DestroyComponent (Variables|Default|GetBox1))
  (Utilities|FlowControl|DoOnce false
    (:Completed
      (Utilities|FlowControl|Sequence
        (:then_0
          (bind _asbp_third_person_character (Utilities|Casting|CastToBP_ThirdPersonCharacter OtherActor))
          (Pawn|Components|CharacterMovement|DisableMovement (Variables|/Script/Engine.Character|GetCharacterMovement _asbp_third_person_character))
          (bind _movecamera (Timeline|Camera%20move Play)
            (:Update
              (Transformation|SetRelativeLocation (Variables|/Game/Blueprints/BP_ThirdPersonCharacter.BP_ThirdPersonCharacter_C|GetFollowCamera _asbp_third_person_character) (Math|Vector|MakeVector (- (.x (Variables|/Script/Engine.SceneComponent|GetRelativeLocation (Variables|/Game/Blueprints/BP_ThirdPersonCharacter.BP_ThirdPersonCharacter_C|GetFollowCamera _asbp_third_person_character))) _movecamera) (.y (Variables|/Script/Engine.SceneComponent|GetRelativeLocation (Variables|/Game/Blueprints/BP_ThirdPersonCharacter.BP_ThirdPersonCharacter_C|GetFollowCamera _asbp_third_person_character))) (+ (.z (Variables|/Script/Engine.SceneComponent|GetRelativeLocation (Variables|/Game/Blueprints/BP_ThirdPersonCharacter.BP_ThirdPersonCharacter_C|GetFollowCamera _asbp_third_person_character))) _movecamera)) false false))))
        (:then_1
          (Utilities|FlowControl|Delay 0.5)
          (bind _drop (Timeline|Timeline_0 Play)
            (:Update
              (Transformation|SetRelativeLocation (Variables|Default|GetFlag) (Math|Vector|MakeVector (.x _relativelocation) (.y _relativelocation) (- (.z _relativelocation) _drop)) false false)
              (Rendering|Material|SetMaterial (Variables|Default|GetFlag) 0 "/Game/LevelPrototyping/Materials/MI_Green.MI_Green"))))
        (:then_2
          (Utilities|FlowControl|Delay 3.0)
          (bind _returnvalue_2 (UserInterface|CreateWidget "/Game/Blueprints/Widgets/WB_Level_Completed_level2.WB_Level_Completed_level2_C" 0 (Variables|Default|GetSeconds)))
          (UserInterface|Viewport|AddtoViewport _returnvalue_2 0)
          (Input|SetInputModeUIOnly _returnvalue _returnvalue_2 "DoNotLock")
          (Variables|/Script/Engine.PlayerController|SetbShowMouseCursor _returnvalue true))))))

(event OnComponentBeginOverlap(Box1)
  (params (OverlappedComponent :type Primitive%20Component%20Object%20Reference) (OtherActor :type Actor%20Object%20Reference) (OtherComp :type Primitive%20Component%20Object%20Reference) (OtherBodyIndex :type Integer) (bFromSweep :type Boolean) (SweepResult :type Hit%20Result%20Structure%20%28by%20ref%29))
  (bind _returnvalue (Game|GetPlayerController 0))
  (bind _flag (Variables|Default|GetFlag))
  (bind _relativelocation (Variables|/Script/Engine.SceneComponent|GetRelativeLocation _flag))
  ;[0.2008 0.6135 0.1357] Here the win-screen is created, we tell it how many seconds it took to complete. Then it's added to the screen and we make sure that the player can see their mouse and restart the level
  (Components|DestroyComponent (Variables|Default|GetBox))
  (Utilities|FlowControl|DoOnce false
    (:Completed
      (Utilities|FlowControl|Sequence
        (:then_0
          (bind _asbp_third_person_character (Utilities|Casting|CastToBP_ThirdPersonCharacter (stale OnComponentBeginOverlap(Box) OtherActor)))
          (Pawn|Components|CharacterMovement|DisableMovement (Variables|/Script/Engine.Character|GetCharacterMovement _asbp_third_person_character))
          (bind _movecamera (Timeline|Camera%20move Play)
            (:Update
              (Transformation|SetRelativeLocation (Variables|/Game/Blueprints/BP_ThirdPersonCharacter.BP_ThirdPersonCharacter_C|GetFollowCamera _asbp_third_person_character) (Math|Vector|MakeVector (- (.x (Variables|/Script/Engine.SceneComponent|GetRelativeLocation (Variables|/Game/Blueprints/BP_ThirdPersonCharacter.BP_ThirdPersonCharacter_C|GetFollowCamera _asbp_third_person_character))) _movecamera) (.y (Variables|/Script/Engine.SceneComponent|GetRelativeLocation (Variables|/Game/Blueprints/BP_ThirdPersonCharacter.BP_ThirdPersonCharacter_C|GetFollowCamera _asbp_third_person_character))) (+ (.z (Variables|/Script/Engine.SceneComponent|GetRelativeLocation (Variables|/Game/Blueprints/BP_ThirdPersonCharacter.BP_ThirdPersonCharacter_C|GetFollowCamera _asbp_third_person_character))) _movecamera)) false false))))
        (:then_1
          (Utilities|FlowControl|Delay 0.5)
          (bind _drop (Timeline|Timeline_0 Play)
            (:Update
              (Transformation|SetRelativeLocation (Variables|Default|GetFlag) (Math|Vector|MakeVector (.x _relativelocation) (.y _relativelocation) (- (.z _relativelocation) _drop)) false false)
              (Rendering|Material|SetMaterial (Variables|Default|GetFlag) 0 "/Game/LevelPrototyping/Materials/MI_Green.MI_Green"))))
        (:then_2
          (Utilities|FlowControl|Delay 3.0)
          (bind _returnvalue_2 (UserInterface|CreateWidget "/Game/Blueprints/Widgets/WB_Level_Completed_Tip.WB_Level_Completed_Tip_C" 0 (Variables|Default|GetSeconds)))
          (UserInterface|Viewport|AddtoViewport _returnvalue_2 0)
          (Input|SetInputModeUIOnly _returnvalue _returnvalue_2 "DoNotLock")
          (Variables|/Script/Engine.PlayerController|SetbShowMouseCursor _returnvalue true))))))

(event Custom|AddSecond
  ;[0.03854 0.03854 0.03854 0.5] This counts the seconds it takes to complete the level
  (Math|Integer|IncrementInt (Variables|Default|GetSeconds)))

(event EventBeginPlay
  ;[0 0.2433 1] Beginplay: When the game starts, this will start an event that counts seconds
  (Utilities|Time|SetTimerbyEvent (delegate Custom|AddSecond) 1.0 true))

(fn ConstructionScript
  (bind _returnvalue (Transformation|GetActorLocation))
  (Transformation|SetActorLocation (Math|Vector|MakeVector 0.0 (.y _returnvalue) (.z _returnvalue)) false true)
  (Transformation|SetActorRotation "0,90.000000, 0"))