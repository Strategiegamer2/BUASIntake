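; Timer Blueprint that runs a minutes-and-seconds countdown and shows the level failed widget when time runs out.
; The Timer flag is cleared at BeginPlay and gates all Tick logic; nothing here sets it true.
; While active, Tick adds a new Timer widget to the viewport each frame, then a one-second Delay paces each decrement.
; Seconds roll over into Minutes, and WB_Level_Failed appears once both are zero.
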(event EventTick
  (params (DeltaSeconds :type Float%20%28single-precision%29))
  (if (Variables|Default|GetTimer)
    (bind _returnvalue (UserInterface|CreateWidget "/Game/Blueprints/Widgets/Timer.Timer_C"))
    (UserInterface|Viewport|AddtoViewport _returnvalue 0)
    (Utilities|FlowControl|Delay 1.0)
    (if (== (Variables|Default|GetSeconds) 0)
      (if (== (Variables|Default|GetMinutes) 0)
        (bind _returnvalue_2 (UserInterface|CreateWidget "/Game/Blueprints/Widgets/WB_Level_Failed.WB_Level_Failed_C"))
        (UserInterface|Viewport|AddtoViewport _returnvalue_2 0)
        (else
          (Variables|Default|SetSeconds 59)
          (Variables|Default|SetMinutes (- (Variables|Default|GetMinutes) 1))))
      (else
        (Variables|Default|SetSeconds (- (Variables|Default|GetSeconds) 1))))))

(event EventBeginPlay
  (Variables|Default|SetTimer false))

(fn ConstructionScript)